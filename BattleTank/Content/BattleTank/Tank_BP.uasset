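; Player-drivable tank Blueprint that wires input to movement, camera aiming and firing.
; On begin play it hands the barrel and turret to the aiming component and both tracks to the movement component.
; Throttle axes drive tracks directly or via movement intents, while aim axes rotate the azimuth gimbal and spring arm.
; Firing spawns Projectile_BP in Blueprint behind a one-second cooldown, leaving TankAiming's Fire call disconnected.
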(event `self.ReceiveBeginPlay`
  (`TankAimingComponent.Initialise` (`self.TankAiming`) (`self.Barrel`) (`self.Turret`))
  (`TankMovementComp.Initialise` (`self.TankMovementComp1`) (`self.TankTrack_L`) (`self.TankTrack_R`)))

(event `InputAxis|Left Track Throttle`
  (params (AxisValue :type "Float (single-precision)"))
  ;[1 1 1] Movement
  (`TankTrack.SetThrottle` (`self.TankTrack_L`) AxisValue))

(event `InputAxis|Right Track Throttle`
  (params (AxisValue :type "Float (single-precision)"))
  ;[1 1 1] Movement
  (`TankTrack.SetThrottle` (`self.TankTrack_R`) AxisValue))

(event `InputAxis|Move Forward`
  (params (AxisValue :type "Float (single-precision)"))
  ;[1 1 1] Movement
  (`TankMovementComp.IntendMoveForward` (`self.TankMovementComp1`) AxisValue))

(event `InputAxis|TurnRight`
  (params (AxisValue :type "Float (single-precision)"))
  ;[1 1 1] Movement
  (`TankMovementComp.IntendTurnRight` (`self.TankMovementComp1`) AxisValue))

(event `InputAxis|AimAzimuth`
  (params (AxisValue :type "Float (single-precision)"))
  ;[1 1 1] Input Binding
  (`SceneComponent.K2_AddLocalRotation` (`self.Azimuth Gimbal`) (`KismetMathLibrary.MakeRotator` 0.0 0.0 (* AxisValue (`GameplayStatics.GetWorldDeltaSeconds`) 100.0)) false false))

(event `InputAxis|AimElevation`
  (params (AxisValue :type "Float (single-precision)"))
  ;[1 1 1] Input Binding
  (`SceneComponent.K2_AddLocalRotation` (`self.SpringArm`) (`KismetMathLibrary.MakeRotator` 0.0 (* AxisValue (`GameplayStatics.GetWorldDeltaSeconds`) 100.0)) false false))

(event `InputAction|Fire`
  (params (Key :type "Key Structure"))
  ;[1 1 1] Input Binding
  (:`Pressed`
    (`self.Firing`)))

(event `Firing`
  (bind _barrel (`self.Barrel`))
  (bind _returnvalue (`SceneComponent.GetSocketRotation` _barrel "None"))
  ;[1 1 1] Fix Fire Rate
  (if (`self.Can Fire`)
    (`|ExecutionSequence`
      (:`then_0`
        (set `self.Can Fire` false)
        (`|SpawnActorFromClass` "/Game/BattleTank/Projectile_BP.Projectile_BP_C" (`KismetMathLibrary.MakeTransform` (+ (`SceneComponent.GetSocketLocation` _barrel "None") (* (`KismetMathLibrary.GetForwardVector` _returnvalue) 800.0)) _returnvalue) "Undefined" "OverrideRootScale" null null))
      (:`then_1`
        (`KismetSystemLibrary.Delay` 1.0)
        (set `self.Can Fire` true)))))

(fn `UserConstructionScript`)